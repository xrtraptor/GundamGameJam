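; Shooter mech enemy that chases the player once seen and fires from a projectile spawn point.
; PawnSensing sets a seen flag and calls FollowPlayer, which moves within range via AIMoveTo, snaps to face the player and spawns an actor.
; Each FollowPlayer call re-arms the attack, and the trailing Delay gates nothing.
; Tick halts movement until the player is seen; sighting is never lost afterwards.
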(event `self.ReceiveTick`
  (params (DeltaSeconds :type "Float (single-precision)"))
  ;[1 1 1] Stop if not seeing Player
  (if (not (`self.isSeeingPlayer`))
    (`MovementComponent.StopMovementImmediately` (`self.CharacterMovement`))))

(event `self.PawnSensing.OnSeePawn`
  (params (Pawn :type "Pawn Object Reference"))
  ;[1 1 1] Search for Player
  (cast `/Game/00_Project/ThirdPerson/Blueprints/BP_ThirdPersonCharacter` Pawn)
  (set `self.isSeeingPlayer` true)
  (`self.FollowPlayer`))

(event `FollowPlayer`
  ;[1 1 1] Attack Player
  (set `self.canAttack` true)
  (if (`self.isSeeingPlayer`)
    (bind _asbp_third_person_character (cast `/Game/00_Project/ThirdPerson/Blueprints/BP_ThirdPersonCharacter` (`GameplayStatics.GetPlayerCharacter` 0)))
    (`|AIMoveTo` self (0.0 0.0 0.0) _asbp_third_person_character 1000.0
      (:`OnSuccess`
        (`self.K2_SetActorRotation` (`KismetMathLibrary.RInterpTo` (`self.K2_GetActorRotation`) (`KismetMathLibrary.FindLookAtRotation` (`self.K2_GetActorLocation`) (`self.K2_GetActorLocation` _asbp_third_person_character)) (`GameplayStatics.GetWorldDeltaSeconds`) 0.0))
        (if (`self.canAttack`)
          (set `self.canAttack` false)
          (`|SpawnActorFromClass` "/Game/00_Project/Misc/BP_Projectile.BP_Projectile_C" (`SceneComponent.K2_GetComponentToWorld` (`self.SpawnProjectileLocation`)) "Undefined" "MultiplyWithRoot" null null)
          (`KismetSystemLibrary.Delay` 1.0))))
    (else
      (set `self.isSeeingPlayer` false))))

(fn `UserConstructionScript`)