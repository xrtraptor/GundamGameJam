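; BP_GundamGameMode is a game mode that holds the count of living enemies and sets up the HUD showing it.
; On BeginPlay it creates WB_HUD, adds it to the viewport, copies NumEnemiesAlive into the enemy counter widget and calls that widget's update event.
; A disconnected chain that would add 10 to the count through a cast of the current game mode never runs.
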(event `self.ReceiveBeginPlay`
  ;[0.1476 0.2144 1] Add Enemies at BeginPlay
  (bind _returnvalue (`|CreateWidget` "/Game/00_Project/02_Widgets/WB_HUD.WB_HUD_C"))
  (bind _output_get (set `self.WHUD` _returnvalue))
  (`UserWidget.AddToViewport` _output_get 0)
  (bind _w_enemycounter (`/Game/00_Project/02_Widgets/WB_HUD.W_EnemyCounter` _output_get))
  (bind _output_get_2 (set `/Game/00_Project/02_Widgets/W_EnemyCounter.NumEnemiesLeft` (`self.NumEnemiesAlive`) _w_enemycounter))
  (`/Game/00_Project/02_Widgets/W_EnemyCounter.CE_UpdateEnemyCounter` _w_enemycounter _output_get_2))

(fn `UserConstructionScript`)